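; Player character Blueprint that handles basic movement and mouse look.
; Forward/back and left/right input axes feed movement input along directions built from the controller's yaw only, so look pitch does not affect movement direction.
; Mouse axes drive controller pitch and yaw, and BeginPlay prints a debug message.
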(event `self.ReceiveBeginPlay`
  (`KismetSystemLibrary.PrintString` "Character Works"))

(event `InputAxis|Button_ForwardBack`
  (params (AxisValue :type "Float (single-precision)"))
  ;[1 1 1] Move Forward and Backward
  (`self.AddMovementInput` (`KismetMathLibrary.GetForwardVector` (`KismetMathLibrary.MakeRotator` 0.0 0.0 (.yaw (`self.GetControlRotation`)))) AxisValue))

(event `InputAxis|Button_LeftRight`
  (params (AxisValue :type "Float (single-precision)"))
  ;[1 1 1] Move Left and Right
  (`self.AddMovementInput` (`KismetMathLibrary.GetRightVector` (`KismetMathLibrary.MakeRotator` 0.0 0.0 (.yaw (`self.GetControlRotation`)))) AxisValue))

(event `InputAxis|Mouse_UpDown`
  (params (AxisValue :type "Float (single-precision)"))
  ;[1 1 1] Moving the Mouse
  (`self.AddControllerPitchInput` AxisValue))

(event `InputAxis|Mouse_LeftRight`
  (params (AxisValue :type "Float (single-precision)"))
  ;[1 1 1] Moving the Mouse
  (`self.AddControllerYawInput` AxisValue))

(fn `UserConstructionScript`)